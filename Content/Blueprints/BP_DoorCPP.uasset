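; Interactable door that opens once by sliding its mesh to a target location with a moving-rock sound.
; Box overlaps set the third-person character's DoorInteract reference to this door on entry and to NewVar0 on exit, with debug prints.
; OpenDoor, which nothing in this graph calls, uses an Opened flag to block repeats and a timeline-driven lerp to move the mesh in relative space.
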(event `self.ReceiveTick`
  (params (DeltaSeconds :type "Float (single-precision)")))

(event `PlaySoundEffect`
  (`GameplayStatics.PlaySoundAtLocation` "/Game/SoundEffect/movingRock.movingRock" (`self.K2_GetActorLocation`) (struct) 1.0 1.0 0.0 null null null))

(event `self.OpenDoor`
  (if (not (`self.opened`))
    (set `self.opened` true)
    (`self.PlaySoundEffect`)
    (bind (_direction _alpha) (`Timeline|Timeline_0`)
      (:`Update`
        (`SceneComponent.K2_SetRelativeLocation` (`self.StaticMesh`) (`KismetMathLibrary.VLerp` (0.0 0.0 0.0) (`self.TargetLocation`) _alpha) false false)))))

(event `self.Box.OnComponentBeginOverlap`
  (params (OverlappedComponent :type "PrimitiveComponent Object Reference") (OtherActor :type "Actor Object Reference") (OtherComp :type "PrimitiveComponent Object Reference") (OtherBodyIndex :type Integer) (bFromSweep :type Boolean) (SweepResult :type "HitResult Structure (by ref)"))
  (bind _astp_third_person_character (cast `TP_ThirdPersonCharacter` OtherActor))
  (set `TP_ThirdPersonCharacter.DoorInteract` self _astp_third_person_character)
  (`KismetSystemLibrary.PrintString` "Set This Door"))

(event `self.Box.OnComponentEndOverlap`
  (params (OverlappedComponent :type "PrimitiveComponent Object Reference") (OtherActor :type "Actor Object Reference") (OtherComp :type "PrimitiveComponent Object Reference") (OtherBodyIndex :type Integer))
  (bind _astp_third_person_character (cast `TP_ThirdPersonCharacter` OtherActor))
  (set `TP_ThirdPersonCharacter.DoorInteract` (`self.NewVar_0`) _astp_third_person_character)
  (`KismetSystemLibrary.PrintString` "Set NULL"))

(fn `UserConstructionScript`)